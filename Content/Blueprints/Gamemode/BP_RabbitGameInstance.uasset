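; BP_RabbitGameInstance is the rabbit game's Game Instance, providing shared helpers for background music and menu-style widgets.
; PlayBackgroundMusic spawns a 2D sound with a given volume and optional persistence across level transitions, storing it in BGM.
; AddWidgetToViewport creates and shows any given widget class, disables input on BP_Rabbit, shows the mouse cursor and switches to UI-only input focused on that widget.
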(event `Play Background Music`
  (params (AudioSource :type "SoundBase Object Reference") (VolumeMultiplier :type "Float (single-precision)") (bPersist :type Boolean))
  (bind _returnvalue (`GameplayStatics.SpawnSound2D` AudioSource VolumeMultiplier 1.0 0.0 null bPersist))
  (set `self.BGM` _returnvalue))

(fn `AddWidgetToViewport`
  (params (Class :type "UserWidget Class Reference"))
  (bind _returnvalue (`|CreateWidget` Class (`GameplayStatics.GetPlayerController` 0)))
  (`UserWidget.AddToViewport` _returnvalue 0)
  (bind _returnvalue_2 (`GameplayStatics.GetActorOfClass` "/Game/Blueprints/Player/BP_Rabbit.BP_Rabbit_C"))
  (`Actor.DisableInput` _returnvalue_2 (`GameplayStatics.GetPlayerController` 0))
  (set `PlayerController.bShowMouseCursor` true (`GameplayStatics.GetPlayerController` 0))
  (`WidgetBlueprintLibrary.SetInputMode_UIOnlyEx` (`GameplayStatics.GetPlayerController` 0) _returnvalue))