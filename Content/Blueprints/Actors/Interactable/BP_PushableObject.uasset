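; BP_PushableObject is an interactable actor that slides toward a new location when a character interacts with it.
; IsInteracted calls CalculateToGoDirection with the character, then plays the ConstantlyMove timeline, using an IsMoving flag to ignore input until it finishes.
; Each update interpolates toward Direction with a swept move, feeding the timeline track into VInterpTo as DeltaTime instead of frame time.
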(event `self.ReceiveTick`
  (params (DeltaSeconds :type "Float (single-precision)")))

(event `InteractableInterface.IsInteracted`
  (params (InCharacter :type "Character Object Reference"))
  ;[1 1 1] E Pressed
  (if (not (`self.bIsMoving`))
    (set `self.bIsMoving` true)
    (`self.CalculateToGoDirection` InCharacter)
    (bind (_direction _newtrack_0) (`Timeline|ConstantlyMove` :!via `PlayFromStart`)
      (:`Update`
        (`self.K2_SetActorLocation` (`KismetMathLibrary.VInterpTo` (`self.K2_GetActorLocation`) (`self.Direction`) _newtrack_0 1.5) true))
      (:`Finished`
        (set `self.bIsMoving` false)))))

(fn `UserConstructionScript`)